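; Enemy AI character Blueprint that writes sight perception of the player into its Blackboard.
; HandleAISense filters for sight stimuli from player 0, then sets TargetActor to the player when sensed or clears it when sight is lost.
; LastKnownLocation updates only on successful sensing, so it persists after the target clears.
; The only HandleAISense call in the EventGraph is unwired, so nothing in this Blueprint triggers it.
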(fn ConstructionScript)

(fn HandleAISense
  (params (Actor :type Actor%20Object%20Reference) (Sense :type AI%20Stimulus%20Structure))
  (bind _stimulus (Variables|Default|GetStimulus))
  (bind _returnvalue (Class|AIPerceptionSystem|GetSenseClassforStimulus (Variables|Default|GetStimulus)))
  (if (== _returnvalue "/Script/AIModule.AISenseConfig_Sight")
    (if (== Actor (Game|GetPlayerCharacter 0))
      (AI|Components|Blackboard|SetValueasObject (AI|GetBlackboard 0) (Utilities|Name|MakeLiteralName "TargetActor") (Utilities|SelectObject (Game|GetPlayerCharacter 0) 0 (.bsuccessfullysensed _stimulus)))
      (if (.bsuccessfullysensed _stimulus)
        (AI|Components|Blackboard|SetValueasVector (AI|GetBlackboard 0) (Utilities|Name|MakeLiteralName "LastKnownLocation") (.stimuluslocation _stimulus)))
      (else
        (return)))
    (else
      (return))))